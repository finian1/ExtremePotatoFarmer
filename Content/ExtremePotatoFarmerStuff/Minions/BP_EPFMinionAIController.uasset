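; AI controller for Extreme Potato Farmer minions that shuttles a minion between its home and work buildings.
; On BeginPlay it casts the controlled pawn to BP_EPFBaseMinion and caches both building locations from its minion stats.
; Two custom events chain AI MoveTo calls, each triggering the other when the move finishes, forming an endless commute while HeadingHome tracks direction.
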(event Custom|GoToWork_Event
  (Variables|Default|SetHeadingHome false)
  (AI|AIMoveTo 0 (Variables|Default|GetWork) 0 -1.0 "Default" "Default" true true
    (:OnMoveFinished
      (CallFunction|GoHomeEvent))))

(event Custom|GoHome_Event
  (Variables|Default|SetHeadingHome true)
  (AI|AIMoveTo 0 (Variables|Default|GetHome) 0 -1.0 "Default" "Default" true true
    (:OnMoveFinished
      (CallFunction|GotoWorkEvent))))

(event EventBeginPlay
  (bind _asbp_epfbase_minion (Utilities|Casting|CastToBP_EPFBaseMinion (Pawn|GetControlledPawn)))
  (Variables|Default|SetHome (Transformation|GetActorLocation (.homeBuilding (Utilities|Struct|BreakMinionStats (Variables|/Script/ExtremePotatoFarmer.EPFBaseMinion|GetmMinionStats _asbp_epfbase_minion)))))
  (Variables|Default|SetWork (Transformation|GetActorLocation (.workBuilding (Utilities|Struct|BreakMinionStats (Variables|/Script/ExtremePotatoFarmer.EPFBaseMinion|GetmMinionStats _asbp_epfbase_minion)))))
  (CallFunction|GotoWorkEvent))

(fn ConstructionScript)