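; AI controller for worker minions in the ExtremePotatoFarmer game that runs an endless commute between home and work buildings.
; On BeginPlay it reads both buildings from the controlled minion's stats, then heads to work.
; Two custom events chain through AIMoveTo: arrival at work calls Work and waits that building's work time before going home, and arrival home restarts the trip.
; A HeadingHome flag records the current direction.
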(event Custom|GoToWork_Event
  (Variables|Default|SetHeadingHome false)
  (AI|AIMoveTo 0 "0, 0, 0" (Variables|Default|GetWorkBuilding) -1.0 "Default" "Default" true true
    (:OnMoveFinished
      (Class|EPFBaseBuilding|Work (Variables|Default|GetWorkBuilding))
      (Utilities|FlowControl|Delay (Variables|/Script/ExtremePotatoFarmer.EPFBaseBuilding|GetmTimeToWork (Variables|Default|GetWorkBuilding)))
      (CallFunction|GoHomeEvent))))

(event Custom|GoHome_Event
  (Variables|Default|SetHeadingHome true)
  (AI|AIMoveTo 0 "0, 0, 0" (Variables|Default|GetHomeBuilding) -1.0 "Default" "Default" true true
    (:OnMoveFinished
      (CallFunction|GotoWorkEvent))))

(event EventBeginPlay
  (bind _asbp_epfbase_minion (Utilities|Casting|CastToBP_EPFBaseMinion (Pawn|GetControlledPawn)))
  (Variables|Default|SetHomeBuilding (.homeBuilding (Utilities|Struct|BreakMinionStats (Variables|/Script/ExtremePotatoFarmer.EPFBaseMinion|GetmMinionStats _asbp_epfbase_minion))))
  (Variables|Default|SetWorkBuilding (.workBuilding (Utilities|Struct|BreakMinionStats (Variables|/Script/ExtremePotatoFarmer.EPFBaseMinion|GetmMinionStats _asbp_epfbase_minion))))
  (CallFunction|GotoWorkEvent))

(fn ConstructionScript)